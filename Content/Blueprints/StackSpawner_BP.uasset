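; StackSpawner_BP is a spawner actor that builds a vertical stack of Tile_BP actors and sends a moving tile out from its side.
; On BeginPlay it spawns tiles at its root, raising the root by a fixed Z step after each one, then calls SpawnTile once.
; SpawnTile creates a tile at LeftSpawner and stores it as CurrentTile, which Tick slides along world X through MoveTile, scaled by delta time.
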(event `self.ReceiveBeginPlay`
  (for _ (range (+ (`self.NumberOfTilesToSpawn`) 1))
    (`|SpawnActorFromClass` "/Game/Blueprints/Tile_BP.Tile_BP_C" (`SceneComponent.K2_GetComponentToWorld` (`self.DefaultSceneRoot`)) "Undefined" "OverrideRootScale" null null)
    (`SceneComponent.K2_AddWorldOffset` (`self.DefaultSceneRoot`) (`KismetMathLibrary.MakeVector` 0.0 0.0 (`self.ZValueDistance`)) false false))
  (`self.SpawnTile`))

(event `SpawnTile`
  (bind _returnvalue (`|SpawnActorFromClass` "/Game/Blueprints/Tile_BP.Tile_BP_C" (`KismetMathLibrary.MakeTransform` (`SceneComponent.K2_GetComponentLocation` (`self.LeftSpawner`))) "Undefined" "OverrideRootScale" null null))
  (set `self.CurrentTile` _returnvalue))

(event `self.ReceiveTick`
  (params (DeltaSeconds :type "Float (single-precision)"))
  (if (`KismetSystemLibrary.IsValid` (`self.CurrentTile`))
    (`self.MoveTile` (`self.CurrentTile`) DeltaSeconds (`self.TileSpeed`))))

(fn `MoveTile`
  (params (`Current Tile` :type "/Game/Blueprints/Tile_BP Object Reference") (DeltaTime :type "Float (double-precision)") (Speed :type "Float (double-precision)"))
  (bind _result (`/Engine/EditorBlueprintResources/StandardMacros.NegateFloat` (* DeltaTime Speed))
    (:`  `
      (`self.K2_AddActorWorldOffset` `Current Tile` (`KismetMathLibrary.MakeVector` _result) false false))))

(fn `UserConstructionScript`)